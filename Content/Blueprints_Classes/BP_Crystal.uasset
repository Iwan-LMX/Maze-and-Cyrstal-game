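; BP_Crystal is a collectible crystal that gets absorbed into the player on overlap, then destroys itself.
; An IsPlayer check gates the overlap, then the starting location, scale and point light intensity are stored.
; A single timeline alpha lerps the crystal toward the player pawn's current location while shrinking it to zero and fading its light.
; The actor is destroyed when the timeline finishes, with no score or inventory update here.
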(event Collision|EventActorBeginOverlap
  (params (OtherActor :type Actor%20Object%20Reference))
  (Utilities|IsPlayer OtherActor
    (:Is%20Player
      (CallFunction|StoreStartingValues)
      (bind _newtrack_0 (Timeline|Alpha%20Blend%20Timeline Play)
        (:Update
          (CallFunction|MovetoPlayer _newtrack_0)
          (CallFunction|ScaleCrystal _newtrack_0)
          (CallFunction|AdjustLight _newtrack_0))
        (:Finished
          (Actor|DestroyActor))))))

(fn ConstructionScript)

(fn MovetoPlayer
  (params (Alpha :type Float%20%28single-precision%29))
  (Transformation|SetActorLocation (Math|Vector|Lerp(Vector) (Variables|Default|GetLerp%20start%20location) (Transformation|GetActorLocation (Game|Player|GetPlayerPawn 0)) Alpha) false false))

(fn StoreStartingValues
  (Variables|Default|SetLerp%20start%20location (Transformation|GetActorLocation))
  (Variables|Default|SetOriginal%20scale (Transformation|GetActorScale3D))
  (Variables|Default|SetStart%20light%20intensity (Variables|/Script/Engine.LightComponentBase|GetIntensity (Variables|Default|GetPointLight))))

(fn ScaleCrystal
  (params (Alpha :type Float%20%28single-precision%29))
  (Transformation|SetActorScale3D (Math|Vector|Lerp(Vector) (Variables|Default|GetOriginal%20scale) "0, 0, 0" Alpha)))

(fn AdjustLight
  (params (Alpha :type Float%20%28double-precision%29))
  (Rendering|Components|Light|SetIntensity (Variables|Default|GetPointLight) (Math|Float|Lerp (Variables|Default|GetStart%20light%20intensity) 0.0 Alpha)))