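; Trigger actor that restarts the current level when the player pawn enters its box, with camera fades for the transition.
; On overlap it fades the camera to a held pale grey, waits for the fade to finish, then reopens the current level by name.
; On BeginPlay it also fades the camera in from full opacity, easing the start of each load.
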(event OnComponentBeginOverlap(Box)
  (params (OverlappedComponent :type Primitive%20Component%20Object%20Reference) (OtherActor :type Actor%20Object%20Reference) (OtherComp :type Primitive%20Component%20Object%20Reference) (OtherBodyIndex :type Integer) (bFromSweep :type Boolean) (SweepResult :type Hit%20Result%20Structure%20%28by%20ref%29))
  ;[1 1 1] Reset level and camera fading
  (if (== OtherActor (Game|Player|GetPlayerPawn 0))
    (CameraFades|StartCameraFade (Game|GetPlayerCameraManager 0) 0.0 1.0 3.0 "(R=0.698661,G=0.703125,B=0.679964,A=1.000000)" false true)
    (Utilities|FlowControl|Delay 3.0)
    (bind _returnvalue (Game|GetCurrentLevelName true))
    (Game|OpenLevel(byName) (Utilities|String|StringToName _returnvalue))))

(event EventBeginPlay
  ;[0.2181 1 0.9702] Game start camera fading
  (CameraFades|StartCameraFade :self (Game|GetPlayerCameraManager 0) :FromAlpha 1.0 :Duration 3.0))

(fn ConstructionScript)