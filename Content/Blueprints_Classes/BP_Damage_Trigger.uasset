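; BP_Damage_Trigger is a box trigger that damages the player on overlap and also starts a camera fade when play begins.
; An Is Player check compares the overlapping actor to player pawn 0, and only a match receives a burst of small ApplyDamage calls from a loop with no delay.
; BeginPlay separately fades player 0's camera from full alpha over a few seconds as a game-start effect.
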(event OnComponentBeginOverlap(Box)
  (params (OverlappedComponent :type Primitive%20Component%20Object%20Reference) (OtherActor :type Actor%20Object%20Reference) (OtherComp :type Primitive%20Component%20Object%20Reference) (OtherBodyIndex :type Integer) (bFromSweep :type Boolean) (SweepResult :type Hit%20Result%20Structure%20%28by%20ref%29))
  ;[1 1 1] Damage to Player
  (Utilities|IsPlayer OtherActor
    (:Is%20Player
      (for _index (range 0 5)
        (Game|Damage|ApplyDamage OtherActor 1.0 0 0)))))

(event EventBeginPlay
  ;[0.2181 1 0.9702] Game start camera fading
  (CameraFades|StartCameraFade :self (Game|GetPlayerCameraManager 0) :FromAlpha 1.0 :Duration 3.0))

(fn ConstructionScript)