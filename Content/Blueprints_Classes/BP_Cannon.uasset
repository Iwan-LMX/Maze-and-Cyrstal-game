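; BP_Cannon is a cannon actor that automatically fires projectiles on a repeating cycle from the start of play.
; After each FireRate delay it spawns a BP_Projectile at the Arrow component's world location and rotation.
; A timeline then slides the Cannon component along its relative Y axis as barrel motion, and its completion loops back to the delay for the next shot.
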(event EventBeginPlay
  (Utilities|FlowControl|Delay (Variables|Default|GetFireRate) :!label _label)
  (CallFunction|SpawnProjectile)
  (bind _newtrack_0 (Timeline|Canon_fire_timeline PlayFromStart)
    (:Update
      (CallFunction|MoveCannonBarrel _newtrack_0))
    (:Finished
      (goto _label))))

(fn ConstructionScript)

(fn SpawnProjectile
  (bind _arrow (Variables|Default|GetArrow))
  (Game|SpawnActorfromClass "/Game/Blueprints_Classes/BP_Projectile.BP_Projectile_C" (Math|Transform|MakeTransform (Transformation|GetWorldLocation _arrow) (Transformation|GetWorldRotation _arrow) "1.000000,1.000000,1.000000") "Undefined" "MultiplyWithRoot" 0 0))

(fn MoveCannonBarrel
  (params (NewLocation_Y :type Float%20%28double-precision%29))
  (Transformation|SetRelativeLocation (Variables|Default|GetCannon) (Math|Vector|MakeVector 0.0 NewLocation_Y 0.0) false false))