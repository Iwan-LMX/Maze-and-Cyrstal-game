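; BP_player is a player that moves by rolling its static mesh with physics torque and restarts the level on death.
; Forward and sideways axis inputs add Y and X torque, scaled by an acceleration multiplier.
; Each damage event costs a life, ignoring damage amount; a hit with none left hides the mesh, disables collision and spawns an explosion.
; After a short delay, Restart The level fades the camera and reopens the current level.
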(event Game|Damage|EventAnyDamage
  (params (Damage :type Float%20%28single-precision%29) (DamageType :type Damage%20Type%20Object%20Reference) (InstigatedBy :type Controller%20Object%20Reference) (DamageCauser :type Actor%20Object%20Reference))
  (if (< (Variables|Default|GetPlayer%20Lives) 1)
    (Rendering|SetVisibility (Variables|Default|GetStaticMesh) false false)
    (Collision|SetCollisionEnabled (Variables|Default|GetStaticMesh) "NoCollision")
    (Effects|SpawnEmitteratLocation "/Game/StarterContent/Particles/P_Explosion.P_Explosion" (Transformation|GetWorldLocation (Variables|Default|GetStaticMesh)))
    (Utilities|FlowControl|Delay 1.0)
    (Utilities|RestarttheLevel)
    (else
      (Variables|Default|SetPlayer%20Lives (+ -1 (Variables|Default|GetPlayer%20Lives))))))

(event Input|AxisEvents|InputAxisMove-forwards-backwards
  (params (AxisValue :type Float%20%28single-precision%29))
  (Class|PrimitiveComponent|AddTorqueinRadians (Variables|Default|GetStaticMesh) (Math|Vector|MakeVector 0.0 (* AxisValue (Variables|Default|GetAcceleration%20multiple)) 0.0) "None" false))

(event Input|AxisEvents|InputAxisMove-right-left
  (params (AxisValue :type Float%20%28single-precision%29))
  (Class|PrimitiveComponent|AddTorqueinRadians (Variables|Default|GetStaticMesh) (Math|Vector|MakeVector (* AxisValue (Variables|Default|GetAcceleration%20multiple)) 0.0 0.0) "None" false))

(fn ConstructionScript)